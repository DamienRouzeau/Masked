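; Zombie enemy that wanders between random reachable points with drunk walk and idle animations.
; AI perception of the first-person player raises its speed and triggers a scream, then a running chase; forgetting the player slows it and re-arms the DoOnce gates.
; PawnSensing hearing sends it toward player noises unless Chasing is set.
; TakeDamage computes Damages minus health, the reverse of the usual order, and calls an empty Die stub.
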(event `ResetPerception`
  (goto _label :!via `Reset`))

(event `self.PawnSensing.OnSeePawn`
  (params (Pawn :type "Pawn Object Reference")))

(event `self.AIPerception.OnTargetPerceptionUpdated`
  (params (Actor :type "Actor Object Reference") (Stimulus :type "AIStimulus Structure"))
  (`KismetSystemLibrary.PrintString` (`KismetSystemLibrary.GetDisplayName` Actor))
  (bind _asbp_first_person_character (cast `/Game/FirstPerson/Blueprints/BP_FirstPersonCharacter` Actor))
  (set `CharacterMovementComponent.MaxWalkSpeed` 820.0 (`self.CharacterMovement`))
  (`/Engine/EditorBlueprintResources/StandardMacros.DoOnce` false :!label _label
    (:`Completed`
      (`SkeletalMeshComponent.PlayAnimation` (`self.Squeleton`) "/Game/Enemies/animation/Zombie_Scream.Zombie_Scream" false)
      (`KismetSystemLibrary.Delay` 2.2)
      (`SkeletalMeshComponent.PlayAnimation` (`self.Squeleton`) "/Game/Enemies/animation/Zombie_Running__1_.Zombie_Running__1_" true)
      (`|AIMoveTo` self (0.0 0.0 0.0) _asbp_first_person_character
        (:`OnSuccess`
          (set `self.Chasing` true))))))

(event `self.PawnSensing.OnHearNoise`
  (params (Instigator :type "Pawn Object Reference") (Location :type "Vector Structure (by ref)") (Volume :type "Float (single-precision)"))
  (cast `/Game/FirstPerson/Blueprints/BP_FirstPersonCharacter` Instigator)
  (if (not (`self.Chasing`))
    (`|AIMoveTo` self Location null)))

(event `self.ReceiveTick`
  (params (DeltaSeconds :type "Float (single-precision)"))
  (`/Engine/EditorBlueprintResources/StandardMacros.DoOnce` false :!label _label_2
    (:`Completed`
      (`SkeletalMeshComponent.PlayAnimation` (`self.Squeleton`) "/Game/Enemies/animation/Drunk_Walk.Drunk_Walk" true :!label _label_3)
      (`|AIMoveTo` self (`NavigationSystemV1.K2_GetRandomReachablePointInRadius` (`self.K2_GetActorLocation`) 2000.0 null null) null
        (:`OnSuccess`
          (`SkeletalMeshComponent.PlayAnimation` (`self.Squeleton`) "/Game/Enemies/animation/Drunk_Idle.Drunk_Idle" true)
          (`KismetSystemLibrary.Delay` (`KismetMathLibrary.RandomFloatInRange` 0.2 10.0))
          (goto _label_3))))))

(event `self.ReceiveBeginPlay`
  (`SkeletalMeshComponent.PlayAnimation` (`self.Squeleton`) "/Game/Enemies/animation/Drunk_Idle.Drunk_Idle" true)
  (goto _label_2))

(event `self.AIPerception.OnTargetPerceptionForgotten`
  (params (Actor :type "Actor Object Reference"))
  (cast `/Game/FirstPerson/Blueprints/BP_FirstPersonCharacter` Actor)
  (`KismetSystemLibrary.PrintString` "lost")
  (`self.ResetPerception`)
  (set `CharacterMovementComponent.MaxWalkSpeed` 130.0 (`self.CharacterMovement`))
  (goto _label_2 :!via `Reset`))

(fn `Die`)

(fn `TakeDamage`
  (params (Damages :type Integer))
  (bind (_name _healths _damage _attackrange _triggerrange) (break `/Game/Enemies/S_Enemies` (`self.enemyStats`)))
  (bind _output_get (set `self.enemyStats` (make `/Game/Enemies/S_Enemies` _name (- Damages _healths) _damage _attackrange _triggerrange)))
  (if (<= (`.Healths_9_19E4A20944DA313CC860D48F8A53C56F` (break `/Game/Enemies/S_Enemies` _output_get)) 0)
    (`self.Die`)))

(fn `UserConstructionScript`
  (`parent.UserConstructionScript`))